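; Player character Blueprint for the Souls project, currently holding only a debug probe for nearby actors.
; Pressing L runs a multi sphere trace by the Pawn profile in a wide radius around the character, ignoring itself and drawing debug shapes.
; Each hit actor's display name is printed.
; An object-type trace node is left unconnected, and the construction script is empty.
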(event EventBeginPlay)

(event Collision|EventActorBeginOverlap
  (params (OtherActor :type Actor%20Object%20Reference)))

(event EventTick
  (params (DeltaSeconds :type Float%20%28single-precision%29)))

(event Input|KeyboardEvents|L
  (params (Key :type Key%20Structure :default "None"))
  (bind _returnvalue (Transformation|GetActorLocation))
  (:Pressed
    (bind (_outhits _returnvalue_2) (Class|KismetSystemLibrary|SphereTraceMultibyProfile _returnvalue _returnvalue 1e+03 "Pawn" true (Utilities|Array|MakeArray self) "ForDuration" true))
    (if _returnvalue_2
      (for _array_element _outhits
        (Development|PrintString (Utilities|GetDisplayName (.HitActor (Collision|BreakHitResult _array_element))))))))

(fn ConstructionScript)